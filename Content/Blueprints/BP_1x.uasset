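; BP_1x is a one-shot point trigger actor that reacts when the first-person character overlaps it, apparently in a level's finish sequence.
; The first such overlap latches Triggered and calls CollideWithPointTrigger on the character, plus StopZipZip if the trigger is flagged LastOne.
; It then checks the character's FinishForce and calls LevelFinished on BP_GameInstance if none remains.
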(event `self.ReceiveBeginPlay`)

(event `self.ReceiveActorBeginOverlap`
  (params (OtherActor :type "Actor Object Reference"))
  (if (not (`self.Triggered`))
    (bind _asbp_first_person_character (cast `/Game/FirstPerson/Blueprints/BP_FirstPersonCharacter` OtherActor))
    (`|ExecutionSequence`
      (:`then_0`
        (set `self.Triggered` true)
        (`ZipZipBallCharacter.CollideWithPointTrigger` _asbp_first_person_character)
        (if (`self.LastOne`)
          (`ZipZipBallCharacter.StopZipZip` _asbp_first_person_character)))
      (:`then_1`
        (if (<= (`ZipZipBallCharacter.FinishForce` _asbp_first_person_character) 0.0)
          (bind _asbp_game_instance (cast `/Game/Blueprints/BP_GameInstance` (`GameplayStatics.GetGameInstance`)))
          (`/Game/Blueprints/BP_GameInstance.LevelFinished` _asbp_game_instance))))))

(fn `UserConstructionScript`)