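; BP_Cubes is an actor holding box meshes that scatter when the first-person character overlaps its Box trigger.
; BeginPlay caches static mesh components tagged "Box", and the overlap pushes each away from the actor origin with partly randomized force.
; CollusionOccured, not called here, spawns and triggers a short-lived, debug-enabled FS_MasterField at a hardcoded location.
; ChangeVisibilirt sets visibility on all cached boxes.
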(event `self.ReceiveBeginPlay`
  (for _array_element (`self.K2_GetComponentsByClass` "/Script/Engine.StaticMeshComponent")
    (if (`ActorComponent.ComponentHasTag` _array_element "Box")
      (`KismetArrayLibrary.Array_Add` (`self.BoxComponents`) _array_element))))

(event `self.Box.OnComponentBeginOverlap`
  (params (OverlappedComponent :type "PrimitiveComponent Object Reference") (OtherActor :type "Actor Object Reference") (OtherComp :type "PrimitiveComponent Object Reference") (OtherBodyIndex :type Integer) (bFromSweep :type Boolean) (SweepResult :type "HitResult Structure (by ref)"))
  (cast `/Game/FirstPerson/Blueprints/BP_FirstPersonCharacter` OtherActor)
  (for _array_element (`self.BoxComponents`)
    (bind _asprimitive_component (cast `PrimitiveComponent` _array_element))
    (`PrimitiveComponent.AddForce` _asprimitive_component (* (- (`SceneComponent.K2_GetComponentLocation` _array_element) (`self.K2_GetActorLocation`)) (* (2500.0 2500.0 2500.0) (* (`KismetMathLibrary.MakeVector` (`KismetMathLibrary.RandomFloatInRange` 0.0 1.0) 1.0 (`KismetMathLibrary.RandomFloatInRange` 0.0 1.0)) (1.0 1.0 1.0)))) "None" false)))

(fn `ChangeVisibilirt`
  (params (Visibility :type Boolean))
  (for _array_element (`self.BoxComponents`)
    (`SceneComponent.SetVisibility` _array_element Visibility false)))

(fn `CollusionOccured`
  (bind _returnvalue (`|SpawnActorFromClass` "/Engine/EditorResources/FieldNodes/FS_MasterField.FS_MasterField_C" (`KismetMathLibrary.MakeTransform` (`KismetMathLibrary.TransformLocation` (`self.GetTransform`) (`KismetMathLibrary.MakeVector` 4940.0 70.0 1560.0)) (struct) (20.0 20.0 20.0)) "Undefined" "OverrideRootScale" null null))
  (set `/Engine/EditorResources/FieldNodes/FS_MasterField.ActivationType` "NewEnumerator4" _returnvalue)
  (set `/Engine/EditorResources/FieldNodes/FS_MasterField.Debug` true _returnvalue)
  (set `/Engine/EditorResources/FieldNodes/FS_MasterField.ShowDebugText` true _returnvalue)
  (set `/Engine/EditorResources/FieldNodes/FS_MasterField.DestroyActor` true _returnvalue)
  (set `/Engine/EditorResources/FieldNodes/FS_MasterField.UseLifespan` true _returnvalue)
  (set `/Engine/EditorResources/FieldNodes/FS_MasterField.FieldLifespan` 0.1 _returnvalue)
  (set `/Engine/EditorResources/FieldNodes/FS_MasterField.Radial Magnitude` 300.0 _returnvalue)
  (`/Engine/EditorResources/FieldNodes/FS_MasterField.CE_Trigger` _returnvalue))

(fn `UserConstructionScript`)