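; LevelFinished is a trigger actor that reacts when an actor overlaps its Box, apparently marking the end of a level.
; The player character starts ZipZip, while a MyAICharacter stops it.
; Any overlapping actor with an SActionComponent also gains the Action_Dance action, with the trigger as instigator.
; Each overlap also turns on cube visibility on the XCreator reference, when it is valid.
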(event `self.Box.OnComponentBeginOverlap`
  (params (OverlappedComponent :type "PrimitiveComponent Object Reference") (OtherActor :type "Actor Object Reference") (OtherComp :type "PrimitiveComponent Object Reference") (OtherBodyIndex :type Integer) (bFromSweep :type Boolean) (SweepResult :type "HitResult Structure (by ref)"))
  (bind _returnvalue (`self.GetComponentByClass` OtherActor "/Script/ZipZipBall.SActionComponent"))
  (`|ExecutionSequence`
    (:`then_0`
      (bind _asbp_first_person_character (cast `/Game/FirstPerson/Blueprints/BP_FirstPersonCharacter` OtherActor)
        (:`then`
          (`ZipZipBallCharacter.StartZipZip` _asbp_first_person_character))
        (:`CastFailed`
          (bind _asmy_aicharacter (cast `MyAICharacter` OtherActor))
          (`MyAICharacter.StopZipZip` _asmy_aicharacter))))
    (:`then_1`
      (`/Engine/EditorBlueprintResources/StandardMacros.IsValid` _returnvalue
        (:`Is Valid`
          (`SActionComponent.AddAction` _returnvalue self "/Game/FirstPerson/Blueprints/Actions/Action_Dance.Action_Dance_C"))))
    (:`then_2`
      (bind _xcreator (`self.XCreator`)
        (:`then`
          (`/Game/Blueprints/XCreator.CubesVisibility` _xcreator true))
        (:`else`)))))

(fn `UserConstructionScript`)