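; Collectable actor whose sphere travels along a spline and is collected by the AI or ZipZipBall character it touches.
; A timeline started on BeginPlay maps its alpha, offset by a random wrapped start phase, to spline distance and moves the sphere with sweep.
; Sphere overlaps call Collided, which passes the actor, its collectable property and a stunned action to that character's Collect.
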(event `self.ReceiveBeginPlay`
  (bind _spline1 (`self.Spline1`))
  (set `self.initDist` (`KismetMathLibrary.RandomFloat`))
  (bind (_direction _alpha) (`Timeline|Timeline_0`)
    (:`Update`
      (`SceneComponent.K2_SetRelativeLocation` (`self.cac1_Sphere002`) (`SplineComponent.GetLocationAtDistanceAlongSpline` _spline1 (`KismetMathLibrary.Lerp` 0.0 (`SplineComponent.GetSplineLength` _spline1) (mod (+ _alpha (`self.initDist`)) 1.0)) "Local") true false))))

(event `self.cac1_Sphere002.OnComponentBeginOverlap`
  (params (OverlappedComponent :type "PrimitiveComponent Object Reference") (OtherActor :type "Actor Object Reference") (OtherComp :type "PrimitiveComponent Object Reference") (OtherBodyIndex :type Integer) (bFromSweep :type Boolean) (SweepResult :type "HitResult Structure (by ref)"))
  (`self.Collided` OtherActor))

(fn `Collided`
  (params (Object :type "Object Object Reference"))
  (bind _collectable_property (`self.Collectable Property`))
  (bind _asmy_aicharacter (cast `MyAICharacter` Object)
    (:`then`
      (`MyAICharacter.Collect` _asmy_aicharacter self _collectable_property "/Game/FirstPerson/Blueprints/Actions/Action_Stunned.Action_Stunned_C"))
    (:`CastFailed`
      (bind _aszip_zip_ball_character (cast `ZipZipBallCharacter` Object))
      (`ZipZipBallCharacter.Collect` _aszip_zip_ball_character self _collectable_property "/Game/FirstPerson/Blueprints/Actions/Action_Stunned.Action_Stunned_C"))))

(fn `UserConstructionScript`)