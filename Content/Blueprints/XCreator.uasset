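; XCreator builds a numbered X axis at BeginPlay from BP_1x child actors spaced along X by Height.
; Each segment shows its Xincrease multiple, gets an XMat dynamic material and a MidPoint custom primitive value proportional to its position within Xmax.
; The final segment is flagged LastOne, and every tenth gets an extra offset child actor.
; Afterwards it calls every BP_Cubes actor to switch visibility off.
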(event `self.ReceiveBeginPlay`
  (`self.CreateNodes` 0))

(fn `CreateNodes`
  (params (FirstIndex :type Integer))
  (bind _returnvalue (`KismetMathLibrary.FTrunc` (/ (`self.Xmax`) (`self.Xincrease`))))
  (`|ExecutionSequence`
    (:`then_0`
      (for _index (range FirstIndex (+ _returnvalue 1))
        (bind _returnvalue_2 (`AddComponent|NODE_AddChildActorComponent-0` :`RelativeTransform` (`KismetMathLibrary.MakeTransform` (`KismetMathLibrary.MakeVector` (* (`self.Height`) _index)))))
        (bind _asbp_1x (cast `/Game/Blueprints/BP_1x` (`ChildActorComponent.ChildActor` _returnvalue_2)))
        (if (== _index _returnvalue)
          (set `/Game/Blueprints/BP_1x.LastOne` true _asbp_1x))
        (`PrimitiveComponent.CreateDynamicMaterialInstance` (`/Game/Blueprints/BP_1x.Plane` _asbp_1x) 0 "/Game/Material/XMat.XMat" "None")
        (bind _returnvalue_3 (* (`self.Xincrease`) _index))
        (`TextRenderComponent.K2_SetText` (`/Game/Blueprints/BP_1x.TextRender` _asbp_1x) (`KismetTextLibrary.Conv_DoubleToText` _returnvalue_3 "HalfToEven" false true 1 324 1))
        (`PrimitiveComponent.SetScalarParameterForCustomPrimitiveData` (`/Game/Blueprints/BP_1x.Plane` _asbp_1x) "MidPoint" (/ _returnvalue_3 (`self.Xmax`)))
        (if (and (== (mod _index 10) 0) (!= _index 0))
          (bind _returnvalue_4 (`AddComponent|NODE_AddChildActorComponent-1` :`self` _asbp_1x :`RelativeTransform` (`KismetMathLibrary.MakeTransform` (-1000.0 0.0 0.0))))
          (`SceneComponent.K2_SetRelativeLocationAndRotation` :`self` _returnvalue_4 :`NewLocation` (-4000.0 0.0 0.0) :`bTeleport` true))))
    (:`then_1`
      (`self.CubesVisibility` false))))

(fn `CubesVisibility`
  (params (Visibility :type Boolean))
  (bind _outactors (`GameplayStatics.GetAllActorsOfClass` "/Game/Blueprints/BP_Cubes.BP_Cubes_C"))
  (for _array_element _outactors
    (`/Game/Blueprints/BP_Cubes.ChangeVisibilirt` _array_element Visibility)))

(fn `UserConstructionScript`)